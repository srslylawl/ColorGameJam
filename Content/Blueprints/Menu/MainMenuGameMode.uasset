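; Game mode for the main menu that keeps running totals of edibles spawned and collected.
; OnEdibleSpawned and OnEdibleCollected add to their totals, then broadcast the recalculated level progress through ProgressUpdate.
; GetProgress stores and returns the collected-to-spawned ratio, or zero while nothing has been collected.
; BeginPlay, Tick and the construction script are empty.
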(fn `GetProgress`
  (returns (ProgressPercent :type "Float (double-precision)"))
  (locals (LevelProgress :type "Float (double-precision)") (RequiredPercent :type "Float (double-precision)" :default 0.1))
  (bind _totalediblescollected (`self.TotalEdiblesCollected`))
  (if (> _totalediblescollected 0)
    (set `local.LevelProgress` (/ (`KismetMathLibrary.Conv_IntToDouble` _totalediblescollected) (`KismetMathLibrary.Conv_IntToDouble` (`self.TotalEdiblesSpawned`))))
    (else
      (set `local.LevelProgress` 0.0)))
  (return (`local.LevelProgress`)))

(fn `OnEdibleCollected`
  (params (Amount :type Integer))
  (set `self.TotalEdiblesCollected` (+ Amount (`self.TotalEdiblesCollected`)))
  (`self.ProgressUpdate` (`self.GetProgress`)))

(fn `OnEdibleSpawned`
  (params (Amount :type Integer))
  (set `self.TotalEdiblesSpawned` (+ Amount (`self.TotalEdiblesSpawned`)))
  (`self.ProgressUpdate` (`self.GetProgress`)))

(fn `UserConstructionScript`)