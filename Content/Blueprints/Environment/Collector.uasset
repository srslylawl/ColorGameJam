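; Collector actor that takes in EdibleObjects of its Red, Blue or Yellow color, or any color when prismatic.
; On Cylinder overlap, the server triggers collection, plays a sound via an S2C event and disables the object's gravity.
; Server Tick pulls queued objects toward SuccPoint, whose overlap destroys them.
; Per-color collision channels are set in BeginPlay because the construction script, which applies debug materials, fails to set them.
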(event `self.ReceiveBeginPlay`
  (bind _returnvalue (enumliteral `ECollisionChannel` "ECC_GameTraceChannel3"))
  (bind _returnvalue_2 (enumliteral `ECollisionChannel` "ECC_GameTraceChannel1"))
  (bind _returnvalue_3 (enumliteral `ECollisionChannel` "ECC_GameTraceChannel2"))
  (bind _succpoint (`self.SuccPoint`))
  (bind _succpoint_2 (`self.SuccPoint`))
  (bind _cylinder (`self.Cylinder`))
  (bind _returnvalue_4 (select `/Game/Blueprints/Edibles/EdibleColor` (`self.Color`) :`NewEnumerator0` "ECC_GameTraceChannel1" :`NewEnumerator1` "ECC_GameTraceChannel2" :`NewEnumerator2` "ECC_GameTraceChannel3" :!type "ECollisionChannel Enum"))
  (if (`self.IsPrismatic`)
    (`PrimitiveComponent.SetCollisionResponseToAllChannels` _cylinder "ECR_Block")
    (`PrimitiveComponent.SetCollisionResponseToChannel` _cylinder _returnvalue_2 "ECR_Overlap")
    (`PrimitiveComponent.SetCollisionResponseToChannel` _cylinder _returnvalue_3 "ECR_Overlap")
    (`PrimitiveComponent.SetCollisionResponseToChannel` _cylinder _returnvalue "ECR_Overlap")
    (`PrimitiveComponent.SetCollisionResponseToChannel` _cylinder "ECC_Camera" "ECR_Ignore")
    (`PrimitiveComponent.SetCollisionResponseToAllChannels` _succpoint_2 "ECR_Block")
    (`PrimitiveComponent.SetCollisionResponseToChannel` _succpoint_2 _returnvalue_2 "ECR_Overlap")
    (`PrimitiveComponent.SetCollisionResponseToChannel` _succpoint_2 _returnvalue_3 "ECR_Overlap")
    (`PrimitiveComponent.SetCollisionResponseToChannel` _succpoint_2 _returnvalue "ECR_Overlap")
    (`PrimitiveComponent.SetCollisionObjectType` _succpoint_2 _returnvalue_2)
    (else
      ;[1 1 1] Set collision response; doesnt work when done in construction script, so we set it here
      (`PrimitiveComponent.SetCollisionResponseToAllChannels` _cylinder "ECR_Block")
      (`PrimitiveComponent.SetCollisionResponseToChannel` _cylinder _returnvalue_4 "ECR_Overlap")
      (`PrimitiveComponent.SetCollisionResponseToChannel` _cylinder "ECC_Camera" "ECR_Ignore")
      (`PrimitiveComponent.SetCollisionResponseToAllChannels` _succpoint "ECR_Block")
      (`PrimitiveComponent.SetCollisionResponseToChannel` _succpoint _returnvalue_4 "ECR_Overlap")
      (`PrimitiveComponent.SetCollisionObjectType` _succpoint _returnvalue_4))))

(event `self.Cylinder.OnComponentBeginOverlap`
  (params (OverlappedComponent :type "PrimitiveComponent Object Reference") (OtherActor :type "Actor Object Reference") (OtherComp :type "PrimitiveComponent Object Reference") (OtherBodyIndex :type Integer) (bFromSweep :type Boolean) (SweepResult :type "HitResult Structure (by ref)"))
  (`/Engine/EditorBlueprintResources/ActorMacros.Switch Has Authority`
    (:`Authority`
      (bind _asedible_object (cast `/Game/Blueprints/Edibles/EdibleObject` OtherActor))
      (bind _output_get (set `self.SoundLocation` (`self.K2_GetActorLocation` OtherActor)))
      (if (or (== (`self.Color`) (`.Color_18_70F373AE4F4C19CEFFB057BB4E4C47BF` (break `/Game/Blueprints/Structs/EdibleIngameReference` (`/Game/Blueprints/Edibles/EdibleObject.EdibleIngameRef` _asedible_object)))) (`self.IsPrismatic`))
        (`/Game/Blueprints/Edibles/EdibleObject.TriggerCollected` _asedible_object)
        (`self.S2C_PlayCollectedSound` _output_get)
        (`KismetArrayLibrary.Array_AddUnique` (`self.ObjectsToSucc`) _asedible_object)
        (bind _staticmeshcomponent (`StaticMeshActor.StaticMeshComponent` _asedible_object))
        (`PrimitiveComponent.SetCollisionResponseToAllChannels` _staticmeshcomponent "ECR_Ignore")
        (`PrimitiveComponent.SetCollisionResponseToChannel` _staticmeshcomponent (select `/Game/Blueprints/Edibles/EdibleColor` (`self.Color`) :`NewEnumerator0` "ECC_GameTraceChannel1" :`NewEnumerator1` "ECC_GameTraceChannel2" :`NewEnumerator2` "ECC_GameTraceChannel3" :!type "ECollisionChannel Enum") "ECR_Overlap")
        (`PrimitiveComponent.SetEnableGravity` _staticmeshcomponent false)
        (`PrimitiveComponent.SetPhysicsLinearVelocity` _staticmeshcomponent (0.0 0.0 0.0) false "None")))))

(event `S2C_PlayCollectedSound`
  (params (Location :type "Vector Structure"))
  (`KismetSystemLibrary.PrintString` "play sound collected")
  (`GameplayStatics.PlaySoundAtLocation` "/Game/SFX/Cues/Cue_EdibleCollected.Cue_EdibleCollected" Location (struct) 1.0 1.0 0.0 "/Game/SFX/EdibleAttenuation.EdibleAttenuation" null null))

(event `self.ReceiveTick`
  (params (DeltaSeconds :type "Float (single-precision)"))
  (`/Engine/EditorBlueprintResources/ActorMacros.Switch Has Authority`
    (:`Authority`
      (for _array_element (`self.ObjectsToSucc`)
        (`PrimitiveComponent.AddForce` (`StaticMeshActor.StaticMeshComponent` _array_element) (* (- (`SceneComponent.K2_GetComponentLocation` (`self.SuccPoint`)) (`SceneComponent.K2_GetComponentLocation` (`StaticMeshActor.StaticMeshComponent` _array_element))) (`self.succForce`)) "None" true)))))

(event `self.SuccPoint.OnComponentBeginOverlap`
  (params (OverlappedComponent :type "PrimitiveComponent Object Reference") (OtherActor :type "Actor Object Reference") (OtherComp :type "PrimitiveComponent Object Reference") (OtherBodyIndex :type Integer) (bFromSweep :type Boolean) (SweepResult :type "HitResult Structure (by ref)"))
  (bind _asedible_object (cast `/Game/Blueprints/Edibles/EdibleObject` OtherActor))
  (`KismetArrayLibrary.Array_RemoveItem` (`self.ObjectsToSucc`) _asedible_object)
  (`self.K2_DestroyActor` _asedible_object))

(fn `SuccObjects`)

(fn `UserConstructionScript`
  (if (`self.IsPrismatic`)
    (`PrimitiveComponent.SetMaterial` (`self.Cylinder`) 0 "/Game/Materials/Debug/DebugMat.DebugMat")
    (else
      (for _array_element (`self.K2_GetComponentsByClass` "/Script/Engine.StaticMeshComponent")
        (`PrimitiveComponent.SetMaterial` _array_element 0 (select `/Game/Blueprints/Edibles/EdibleColor` (`self.Color`) :`NewEnumerator0` "/Game/Materials/Debug/DebugMatRed.DebugMatRed" :`NewEnumerator1` "/Game/Materials/Debug/DebugMatBlue.DebugMatBlue" :`NewEnumerator2` "/Game/Materials/Debug/DebugMatYellow.DebugMatYellow" :!type "MaterialInterface Object Reference"))))))