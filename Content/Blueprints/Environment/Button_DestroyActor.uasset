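; A one-shot trigger button that destroys a referenced actor, ActorToDestroy, when the MainCharacter overlaps it.
; The construction script applies the inactive material, and the trigger overlap calls Activate, guarded by IsActive so it runs only once.
; Activate swaps to the active material, caches the target's location, destroys it, then plays a 2D secret cue and calls a positional sound at the cached location.
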(event `self.Trigger.OnComponentBeginOverlap`
  (params (OverlappedComponent :type "PrimitiveComponent Object Reference") (OtherActor :type "Actor Object Reference") (OtherComp :type "PrimitiveComponent Object Reference") (OtherBodyIndex :type Integer) (bFromSweep :type Boolean) (SweepResult :type "HitResult Structure (by ref)"))
  (if (not (`self.IsActive`))
    (cast `/Game/Blueprints/Character/SlimeCharacter/MainCharacter` OtherActor)
    (`self.Activate`)))

(fn `Activate`
  (bind _actortodestroy (`self.ActorToDestroy`))
  (if (not (`self.IsActive`))
    (set `self.IsActive` true)
    (`PrimitiveComponent.SetMaterial` (`self.StaticMesh`) 0 (`self.ActiveMat`))
    (bind _output_get (set `self.SoundLocation` (`self.K2_GetActorLocation` _actortodestroy)))
    (`self.K2_DestroyActor` _actortodestroy)
    (`GameplayStatics.PlaySound2D` "/Game/SFX/Cues/Cue_Secret.Cue_Secret" 1.0 1.0 0.0 null null)
    (`GameplayStatics.PlaySoundAtLocation` null _output_get (struct) 1.0 1.0 0.0 null null null)))

(fn `UserConstructionScript`
  (`PrimitiveComponent.SetMaterial` (`self.StaticMesh`) 0 (`self.InactiveMat`)))