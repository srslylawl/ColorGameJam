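; OMNIBOOST is an environment boost actor that speeds up overlapping bumpable objects along their current direction of travel.
; On overlap it gets the physics object through IBumpable, applies a velocity-change impulse, optionally plays a sound, notifies the bumpable and starts a cooldown.
; The impulse follows the normalized velocity, optionally flattened to horizontal, scaled by force settings.
; The construction script applies an optional decal material.
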(event `self.ReceiveActorBeginOverlap`
  (params (OtherActor :type "Actor Object Reference"))
  (bind _cue (`self.Cue`))
  (bind _asibumpable (cast `/Game/Blueprints/Environment/IBumpable` OtherActor))
  (if (`self.Ready`)
    (bind _object (`/Game/Blueprints/Environment/IBumpable.GetObjectToBump` _asibumpable))
    (`self.Boost` _object)
    (if (`self.PlayCue`)
      (`/Engine/EditorBlueprintResources/StandardMacros.IsValid` _cue
        (:`Is Valid`
          (`GameplayStatics.PlaySoundAtLocation` _cue (`self.K2_GetActorLocation`) (struct) 1.0 1.0 0.0 "/Game/SFX/EdibleAttenuation.EdibleAttenuation" null null))
        (:`Is Not Valid`
          _)))
    (`/Game/Blueprints/Environment/IBumpable.OnBumped` _asibumpable)
    (set `self.Ready` false)
    (`KismetSystemLibrary.Delay` (`self.Cooldown`))
    (set `self.Ready` true)))

(fn `Boost`
  (params (ObjectToBoost :type "PrimitiveComponent Object Reference"))
  (bind _returnvalue (`PrimitiveComponent.GetPhysicsLinearVelocity` ObjectToBoost "None"))
  (if (`self.HorizontalOnly`)
    (`PrimitiveComponent.AddImpulse` ObjectToBoost (* (* (`KismetMathLibrary.Normal` (`KismetMathLibrary.MakeVector` (.x _returnvalue) (.y _returnvalue))) (`self.Force`)) (`self.ForceMultiplier`)) "None" true)
    (else
      (`PrimitiveComponent.AddImpulse` ObjectToBoost (* (* (`KismetMathLibrary.Normal` _returnvalue) (`self.Force`)) (`self.ForceMultiplier`)) "None" true))))

(fn `UserConstructionScript`
  (`/Engine/EditorBlueprintResources/StandardMacros.IsValid` (`self.DecalMaterial`)
    (:`Is Valid`
      (`DecalComponent.SetDecalMaterial` (`self.Decal`) (`self.DecalMaterial`)))))