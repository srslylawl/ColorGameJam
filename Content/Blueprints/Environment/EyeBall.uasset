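; Eyeball environment actor that watches a MainCharacter inside its Radius sphere and shows anger with a rotating brow, mirrorable for either side.
; Sphere overlap sets the tracked player, though its closer-player check compares the root to itself, so it never switches from a valid target.
; Each tick eases the eye toward that player within MaxAngle, otherwise forward, tilts the brow angry or neutral, and draws a debug point at the look target.
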(event `self.ReceiveTick`
  (params (DeltaSeconds :type "Float (single-precision)"))
  (`self.TrackPlayer`)
  (`self.LookAt` DeltaSeconds)
  (`self.ChangeExpression` DeltaSeconds)
  (`KismetSystemLibrary.DrawDebugPoint` (`self.LookAtLocation`) 50.0 (struct :`R` 0.122709 :`G` 0.37721 :`B` 1.0 :`A` 1.0)))

(event `self.Radius.OnComponentBeginOverlap`
  (params (OverlappedComponent :type "PrimitiveComponent Object Reference") (OtherActor :type "Actor Object Reference") (OtherComp :type "PrimitiveComponent Object Reference") (OtherBodyIndex :type Integer) (bFromSweep :type Boolean) (SweepResult :type "HitResult Structure (by ref)"))
  (bind _trackedplayer (`self.TrackedPlayer`))
  (bind _defaultsceneroot (`self.DefaultSceneRoot`))
  (bind _asmain_character (cast `/Game/Blueprints/Character/SlimeCharacter/MainCharacter` OtherActor))
  (if (`self.TrackClosestPlayer`)
    (`/Engine/EditorBlueprintResources/StandardMacros.IsValid` _trackedplayer
      (:`Is Valid`
        (if (!= _trackedplayer _asmain_character)
          (if (< (`KismetMathLibrary.Vector_DistanceSquared` (`SceneComponent.K2_GetComponentLocation` (`/Game/Blueprints/Character/SlimeCharacter/MainCharacter.SkeletalMesh` _trackedplayer)) (`SceneComponent.K2_GetComponentLocation` (`self.DefaultSceneRoot`))) (`KismetMathLibrary.Vector_DistanceSquared` (`SceneComponent.K2_GetComponentLocation` _defaultsceneroot) (`SceneComponent.K2_GetComponentLocation` _defaultsceneroot)))
            (set `self.TrackedPlayer` _asmain_character))))
      (:`Is Not Valid`
        (set `self.TrackedPlayer` _asmain_character)))))

(fn `ChangeExpression`
  (params (deltaTime :type "Float (double-precision)"))
  (locals (AngryFace :type "Rotator Structure" :default (struct :`Roll` 15.0)) (NeutralFace :type "Rotator Structure" :default (struct :`Roll` -15.00007)) (DesiredExpression :type "Rotator Structure"))
  (bind _brow (`self.brow`))
  (bind (_returnvalue_location _returnvalue_rotation) (`KismetMathLibrary.BreakTransform` (`SceneComponent.GetRelativeTransform` _brow)))
  (if (`self.Mirror`)
    (set `local.AngryFace` (struct :`Roll` -15.0))
    (set `local.NeutralFace` (struct :`Roll` 15.0))
    (else
      (set `local.AngryFace` (struct :`Roll` 15.0))
      (set `local.NeutralFace` (struct :`Roll` -15.0))))
  (if (`self.IsAngry`)
    (set `local.DesiredExpression` (`local.AngryFace`))
    (else
      (set `local.DesiredExpression` (`local.NeutralFace`))))
  (`SceneComponent.K2_SetRelativeRotation` _brow (`KismetMathLibrary.RLerp` _returnvalue_rotation (`local.DesiredExpression`) (* deltaTime 3.0) true) false false))

(fn `LookAt`
  (params (deltaTime :type "Float (double-precision)"))
  (locals (targetVec :type "Rotator Structure") (forward :type "Vector Structure" :default (1.0 0.0 0.0)))
  (bind _eye (`self.Eye`))
  (bind _returnvalue (`KismetMathLibrary.Normal` (- (`self.LookAtLocation`) (`SceneComponent.K2_GetComponentLocation` _eye))))
  (bind _output_get (set `local.forward` (`SceneComponent.GetForwardVector` (`self.Arrow`))))
  (if (<= (`KismetMathLibrary.DegAcos` (`KismetMathLibrary.Dot_VectorVector` _returnvalue _output_get)) (`self.MaxAngle`))
    (set `local.targetVec` (`KismetMathLibrary.Conv_VectorToRotator` _returnvalue))
    (else
      (set `local.targetVec` (`KismetMathLibrary.Conv_VectorToRotator` _output_get))))
  (`SceneComponent.K2_SetWorldRotation` (`self.Eye`) (`KismetMathLibrary.RLerp` (`SceneComponent.K2_GetComponentRotation` _eye) (`local.targetVec`) (* deltaTime (`self.TrackSpeed`)) true) false false))

(fn `TrackPlayer`
  (bind _trackedplayer (`self.TrackedPlayer`))
  (bind _returnvalue (`SceneComponent.K2_GetComponentLocation` (`/Game/Blueprints/Character/SlimeCharacter/MainCharacter.SkeletalMesh` _trackedplayer)))
  (if (`self.TrackClosestPlayer`)
    (`/Engine/EditorBlueprintResources/StandardMacros.IsValid` _trackedplayer
      (:`Is Valid`
        (if (<= (`KismetMathLibrary.Vector_DistanceSquared` (`SceneComponent.K2_GetComponentLocation` (`self.Radius`)) _returnvalue) (`KismetMathLibrary.Square` (`SphereComponent.GetScaledSphereRadius` (`self.Radius`))))
          (set `self.LookAtLocation` _returnvalue)
          (set `self.IsAngry` true)
          (else
            (set `self.LookAtLocation` (+ (`SceneComponent.K2_GetComponentLocation` (`self.DefaultSceneRoot`)) (`SceneComponent.GetForwardVector` (`self.Arrow`))) :!label _label)
            (set `self.IsAngry` false))))
      (:`Is Not Valid`
        (goto _label)))
    (else
      (goto _label))))

(fn `UserConstructionScript`
  (bind _brow (`self.brow`))
  (bind (_returnvalue_x _returnvalue_y _returnvalue_z) (`KismetMathLibrary.BreakVector` (`SceneComponent.K2_GetComponentScale` _brow)))
  (set `self.LookAtLocation` (+ (`SceneComponent.K2_GetComponentLocation` (`self.DefaultSceneRoot`)) (`SceneComponent.GetForwardVector` (`self.Arrow`))))
  (if (`self.Mirror`)
    (`SceneComponent.SetWorldScale3D` _brow (`KismetMathLibrary.MakeVector` _returnvalue_x (- 0.0 _returnvalue_y) _returnvalue_z))
    (else
      (`SceneComponent.SetWorldScale3D` _brow (`KismetMathLibrary.MakeVector` _returnvalue_x (`KismetMathLibrary.Abs` _returnvalue_y) _returnvalue_z)))))