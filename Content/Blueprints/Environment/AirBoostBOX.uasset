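; AirBoostBOX is an environment boost trigger that launches overlapping bumpable physics objects along its arrow's forward direction.
; On overlap it gets the target through the IBumpable interface, then a mode applies either a fixed impulse, an impulse scaled by alignment with current velocity, or a velocity override.
; A Ready flag and delay enforce a cooldown between boosts, with an optional 2D sound cue on firing.
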(event `self.ReceiveActorBeginOverlap`
  (params (OtherActor :type "Actor Object Reference"))
  (bind _cue (`self.Cue`))
  (bind _asibumpable (cast `/Game/Blueprints/Environment/IBumpable` OtherActor))
  (if (`self.Ready`)
    (bind _object (`/Game/Blueprints/Environment/IBumpable.GetObjectToBump` _asibumpable))
    (switch `/Game/Blueprints/Environment/BoostMode` (`self.Mode`)
      (:`NewEnumerator0`
        (`self.RelativeBoost` _object))
      (:`NewEnumerator1`
        (`self.FixedBoost` _object))
      (:`NewEnumerator2`
        (`self.OverrideBoost` _object)))
    (if (`self.PlayCue`)
      (`/Engine/EditorBlueprintResources/StandardMacros.IsValid` _cue
        (:`Is Valid`
          (`GameplayStatics.PlaySound2D` _cue 1.0 1.0 0.0 null null))
        (:`Is Not Valid`
          _)))
    (set `self.Ready` false)
    (`KismetSystemLibrary.Delay` (`self.Cooldown`))
    (set `self.Ready` true)))

(fn `FixedBoost`
  (params (ObjectToBoost :type "PrimitiveComponent Object Reference"))
  (`PrimitiveComponent.AddImpulse` ObjectToBoost (* (* (`SceneComponent.GetForwardVector` (`self.Arrow`)) (`self.Force`)) (`self.ForceMultiplier`)) "None" true))

(fn `OverrideBoost`
  (params (ObjectToBoost :type "PrimitiveComponent Object Reference"))
  (`PrimitiveComponent.SetPhysicsLinearVelocity` ObjectToBoost (* (* (`SceneComponent.GetForwardVector` (`self.Arrow`)) (`self.Force`)) (`self.ForceMultiplier`)) false "None"))

(fn `RelativeBoost`
  (params (ObjectToBoost :type "PrimitiveComponent Object Reference"))
  (bind _returnvalue (`SceneComponent.GetForwardVector` (`self.Arrow`)))
  (bind _returnvalue_2 (`PrimitiveComponent.GetPhysicsLinearVelocity` ObjectToBoost "None"))
  (`PrimitiveComponent.AddImpulse` ObjectToBoost (* (* (* _returnvalue (`self.Force`)) (`self.ForceMultiplier`)) (`KismetMathLibrary.FMax` (`KismetMathLibrary.Dot_VectorVector` (`KismetMathLibrary.Normal` _returnvalue_2) _returnvalue))) "None" true))

(fn `UserConstructionScript`)