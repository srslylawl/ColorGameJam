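; FindPathPoint is a Behavior Tree task that sets the location of an AI character's current patrol point.
; It reads an index from the Blackboard and looks up that entry in the PatrolPath points of the controlled AI_Character.
; The point is transformed by the character's own actor transform, written to a Blackboard vector key, and the task finishes successfully.
; If the pawn cast fails, the task never calls FinishExecute.
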(event `self.ReceiveExecuteAI`
  (params (OwnerController :type "AIController Object Reference") (ControlledPawn :type "Pawn Object Reference"))
  ;[1 1 1] Gets us the the path we are currently on
  (bind _asai_character (cast `/Game/Blueprints/AI/AI_Character` ControlledPawn))
  (`BTFunctionLibrary.SetBlackboardValueAsVector` (`self.BB_PathVector`) (`KismetMathLibrary.TransformLocation` (`Actor.GetTransform` _asai_character) (`|GetArrayItem` (`/Game/Blueprints/AI/PatrolPath.PathPoints` (`/Game/Blueprints/AI/AI_Character.PatrolPath` _asai_character)) (`BTFunctionLibrary.GetBlackboardValueAsInt` (`self.BB_PathIndex`)))))
  (`self.FinishExecute` true))