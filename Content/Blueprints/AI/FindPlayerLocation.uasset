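; Behavior tree task that picks a navigable destination near a Slimey actor for the AI to use.
; It loops over all Slimey actors, storing the one closest to the controlled pawn within the persistent Closest threshold.
; It then writes a random navigable point around the loop's last element, rather than the stored closest actor, to a Blackboard vector and finishes successfully.
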(event `self.ReceiveExecuteAI`
  (params (OwnerController :type "AIController Object Reference") (ControlledPawn :type "Pawn Object Reference"))
  (bind _outactors (`GameplayStatics.GetAllActorsOfClass` "/Game/Blueprints/Character/Slimey.Slimey_C"))
  (for _array_element _outactors
    (bind _returnvalue (`Actor.GetDistanceTo` ControlledPawn _array_element))
    (if (<= _returnvalue (`self.Closest`))
      (set `self.Closest` _returnvalue)
      (set `self.Slimey` _array_element)))
  (`BTFunctionLibrary.SetBlackboardValueAsVector` (`self.Vector`) (`NavigationSystemV1.K2_GetRandomLocationInNavigableRadius` (`SceneComponent.K2_GetComponentLocation` (`Actor.RootComponent` _array_element)) 100.0 null null))
  (`self.FinishExecute` true))