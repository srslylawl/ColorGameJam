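; AI controller for AI_Character pawns that combines a patrol behavior tree setup with random wandering.
; On BeginPlay it runs AI_BT, caches the pawn and copies its patrol path's looping flag into the PathLooping blackboard key.
; Separately from the tree, Tick picks a random reachable point and moves to it whenever the pawn is within tolerance of its current Target.
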(event `self.ReceiveBeginPlay`
  (`self.RunBehaviorTree` "/Game/Blueprints/AI/AI_BT.AI_BT")
  (bind _asai_character (cast `/Game/Blueprints/AI/AI_Character` (`self.K2_GetPawn`)))
  ;[1 1 1] is looping gets fed into the blackboard at the start of the game
  (bind _output_get (set `self.MyPawn` _asai_character))
  (`BlackboardComponent.SetValueAsBool` (`AIBlueprintHelperLibrary.GetBlackboard` null) "PathLooping" (`/Game/Blueprints/AI/PatrolPath.IsLooping` (`/Game/Blueprints/AI/AI_Character.PatrolPath` _output_get))))

(event `self.ReceiveTick`
  (params (DeltaSeconds :type "Float (single-precision)"))
  (if (== (`self.Target`) (`self.K2_GetActorLocation` (`self.K2_GetPawn`)) :`ErrorTolerance` 250.0)
    (bind _output_get (set `self.Target` (`NavigationSystemV1.K2_GetRandomReachablePointInRadius` (0.0 0.0 0.0) 1000.0 null null)))
    (`self.MoveToLocation` _output_get -1.0 true true false true null)))

(fn `UserConstructionScript`)