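; Enemy AI controller that runs the Enemy_BT behavior tree for a patrolling enemy.
; On BeginPlay it casts its pawn to Enemy and seeds the blackboard with the patrol path's looping flag, a starting direction and the player-collision flag.
; AI Perception updates set CanSeePlayer whenever the MainCharacter is sensed or lost.
; An older line-of-sight check for the same key is left disconnected.
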(event `self.ReceiveBeginPlay`
  (bind _returnvalue (`AIBlueprintHelperLibrary.GetBlackboard` null))
  (`self.RunBehaviorTree` "/Game/Blueprints/AI/Enemy_BT.Enemy_BT")
  (bind _asenemy (cast `/Game/Blueprints/Character/Enemy` (`self.K2_GetPawn`)))
  (bind _output_get (set `self.MyPawn` _asenemy))
  ;[1 1 1] is looping gets fed in to the blackboard at the start of the game
  (`BlackboardComponent.SetValueAsBool` _returnvalue "PathLooping" (`/Game/Blueprints/AI/PatrolPath.IsLooping` (`/Game/Blueprints/Character/Enemy.PatrolPath` _output_get)))
  (`BlackboardComponent.SetValueAsInt` (`AIBlueprintHelperLibrary.GetBlackboard` null) "Direction" 1)
  (`BlackboardComponent.SetValueAsBool` _returnvalue "CollidedWithPlayer" (`/Game/Blueprints/Character/Enemy.CollidedWithPlayer` (`self.MyPawn`))))

(event `self.AIPerception.OnTargetPerceptionUpdated`
  (params (Actor :type "Actor Object Reference") (Stimulus :type "AIStimulus Structure"))
  (cast `/Game/Blueprints/Character/SlimeCharacter/MainCharacter` Actor)
  (`BlackboardComponent.SetValueAsBool` (`AIBlueprintHelperLibrary.GetBlackboard` null) "CanSeePlayer" (`.bSuccessfullySensed` (break `AIStimulus` Stimulus))))

(fn `UserConstructionScript`)