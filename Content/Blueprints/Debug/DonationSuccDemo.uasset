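; Debug demo of a color-coded suction receptacle that collects EdibleObjects matching its Red, Blue or Yellow setting, which also picks its debug material and collision channel.
; Cylinder overlap triggers collection and sound, then disables the edible's gravity and most collisions.
; Tick pulls collected edibles toward SuccPoint with distance-scaled acceleration.
; An edible overlapping SuccPoint leaves the pull list, and DestroyActor runs on the receptacle itself.
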(event `self.ReceiveBeginPlay`
  (bind _succpoint (`self.SuccPoint`))
  (bind _cylinder (`self.Cylinder`))
  (bind _returnvalue (select `/Game/Blueprints/Edibles/EdibleColor` (`self.Color`) :`NewEnumerator0` "ECC_GameTraceChannel1" :`NewEnumerator1` "ECC_GameTraceChannel2" :`NewEnumerator2` "ECC_GameTraceChannel3" :!type "ECollisionChannel Enum"))
  ;[1 1 1] Set collision response; doesnt work when done in construction script, so we set it here
  (`PrimitiveComponent.SetCollisionResponseToAllChannels` _cylinder "ECR_Block")
  (`PrimitiveComponent.SetCollisionResponseToChannel` _cylinder _returnvalue "ECR_Overlap")
  (`PrimitiveComponent.SetCollisionResponseToChannel` _cylinder "ECC_Camera" "ECR_Ignore")
  (`PrimitiveComponent.SetCollisionResponseToAllChannels` _succpoint "ECR_Block")
  (`PrimitiveComponent.SetCollisionResponseToChannel` _succpoint _returnvalue "ECR_Overlap")
  (`PrimitiveComponent.SetCollisionObjectType` _succpoint _returnvalue))

(event `self.Cylinder.OnComponentBeginOverlap`
  (params (OverlappedComponent :type "PrimitiveComponent Object Reference") (OtherActor :type "Actor Object Reference") (OtherComp :type "PrimitiveComponent Object Reference") (OtherBodyIndex :type Integer) (bFromSweep :type Boolean) (SweepResult :type "HitResult Structure (by ref)"))
  (bind _asedible_object (cast `/Game/Blueprints/Edibles/EdibleObject` OtherActor))
  (bind _output_get (set `self.SoundLocation` (`self.K2_GetActorLocation` OtherActor)))
  (if (== (`self.Color`) (`.Color_18_70F373AE4F4C19CEFFB057BB4E4C47BF` (break `/Game/Blueprints/Structs/EdibleIngameReference` (`/Game/Blueprints/Edibles/EdibleObject.EdibleIngameRef` _asedible_object))))
    (`/Game/Blueprints/Edibles/EdibleObject.TriggerCollected` _asedible_object)
    (`GameplayStatics.PlaySoundAtLocation` "/Game/SFX/Cues/Cue_EdibleCollected.Cue_EdibleCollected" _output_get (struct) 1.0 1.0 0.0 null null null)
    (`KismetArrayLibrary.Array_AddUnique` (`self.ObjectsToSucc`) _asedible_object)
    (bind _staticmeshcomponent (`StaticMeshActor.StaticMeshComponent` _asedible_object))
    (`PrimitiveComponent.SetCollisionResponseToAllChannels` _staticmeshcomponent "ECR_Ignore")
    (`PrimitiveComponent.SetCollisionResponseToChannel` _staticmeshcomponent (select `/Game/Blueprints/Edibles/EdibleColor` (`self.Color`) :`NewEnumerator0` "ECC_GameTraceChannel1" :`NewEnumerator1` "ECC_GameTraceChannel2" :`NewEnumerator2` "ECC_GameTraceChannel3" :!type "ECollisionChannel Enum") "ECR_Overlap")
    (`PrimitiveComponent.SetEnableGravity` _staticmeshcomponent false)
    (`PrimitiveComponent.SetPhysicsLinearVelocity` _staticmeshcomponent (0.0 0.0 0.0) false "None")))

(event `self.ReceiveTick`
  (params (DeltaSeconds :type "Float (single-precision)"))
  (for _array_element (`self.ObjectsToSucc`)
    (`PrimitiveComponent.AddForce` (`StaticMeshActor.StaticMeshComponent` _array_element) (* (- (`SceneComponent.K2_GetComponentLocation` (`self.SuccPoint`)) (`SceneComponent.K2_GetComponentLocation` (`StaticMeshActor.StaticMeshComponent` _array_element))) (`self.succForce`)) "None" true)))

(event `self.SuccPoint.OnComponentBeginOverlap`
  (params (OverlappedComponent :type "PrimitiveComponent Object Reference") (OtherActor :type "Actor Object Reference") (OtherComp :type "PrimitiveComponent Object Reference") (OtherBodyIndex :type Integer) (bFromSweep :type Boolean) (SweepResult :type "HitResult Structure (by ref)"))
  (bind _asedible_object (cast `/Game/Blueprints/Edibles/EdibleObject` OtherActor))
  (`KismetArrayLibrary.Array_RemoveItem` (`self.ObjectsToSucc`) _asedible_object)
  (`self.K2_DestroyActor`))

(fn `SuccObjects`)

(fn `UserConstructionScript`
  (for _array_element (`self.K2_GetComponentsByClass` "/Script/Engine.StaticMeshComponent")
    (`PrimitiveComponent.SetMaterial` _array_element 0 (select `/Game/Blueprints/Edibles/EdibleColor` (`self.Color`) :`NewEnumerator0` "/Game/Debug/DebugMatRed.DebugMatRed" :`NewEnumerator1` "/Game/Debug/DebugMatBlue.DebugMatBlue" :`NewEnumerator2` "/Game/Debug/DebugMatYellow.DebugMatYellow" :!type "MaterialInterface Object Reference"))))