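; DonationBoxDemo is a debug demo of a color-coded donation box that collects edible objects of its own color.
; The construction script applies the debug material for its Color to every static mesh component.
; On BeginPlay, InputCollider blocks all channels except that color's trace channel, set here because it fails in the construction script.
; An overlapping EdibleObject triggers its collected logic if its color matches the box's.
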(event `self.ReceiveBeginPlay`
  (bind _inputcollider (`self.InputCollider`))
  ;[1 1 1] Set collision response; doesnt work when done in construction script, so we set it here
  (`PrimitiveComponent.SetCollisionResponseToAllChannels` _inputcollider "ECR_Block")
  (`PrimitiveComponent.SetCollisionResponseToChannel` _inputcollider (select `/Game/Blueprints/Edibles/EdibleColor` (`self.Color`) :`NewEnumerator0` "ECC_GameTraceChannel1" :`NewEnumerator1` "ECC_GameTraceChannel2" :`NewEnumerator2` "ECC_GameTraceChannel3" :!type "ECollisionChannel Enum") "ECR_Overlap"))

(event `self.InputCollider.OnComponentBeginOverlap`
  (params (OverlappedComponent :type "PrimitiveComponent Object Reference") (OtherActor :type "Actor Object Reference") (OtherComp :type "PrimitiveComponent Object Reference") (OtherBodyIndex :type Integer) (bFromSweep :type Boolean) (SweepResult :type "HitResult Structure (by ref)"))
  (bind _asedible_object (cast `/Game/Blueprints/Edibles/EdibleObject` OtherActor))
  (if (== (`self.Color`) (`.Color_18_70F373AE4F4C19CEFFB057BB4E4C47BF` (break `/Game/Blueprints/Edibles/EdibleIngameReference` (`/Game/Blueprints/Edibles/EdibleObject.EdibleIngameRef` _asedible_object))))
    (`/Game/Blueprints/Edibles/EdibleObject.TriggerCollected` _asedible_object)))

(fn `UserConstructionScript`
  (for _array_element (`self.K2_GetComponentsByClass` "/Script/Engine.StaticMeshComponent")
    (`PrimitiveComponent.SetMaterial` _array_element 0 (select `/Game/Blueprints/Edibles/EdibleColor` (`self.Color`) :`NewEnumerator0` "/Game/Debug/DebugMatRed.DebugMatRed" :`NewEnumerator1` "/Game/Debug/DebugMatBlue.DebugMatBlue" :`NewEnumerator2` "/Game/Debug/DebugMatGreen.DebugMatGreen" :!type "MaterialInterface Object Reference"))))