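; Debug actor that visualizes surface normals of geometry around its sphere component.
; Each Tick, a sphere overlap helper gathers hits, and a line trace against WorldStatic objects runs from the center toward each impact point, scaled to the radius.
; Each trace's impact normal is drawn as a debug arrow from the sphere center.
; The blocking-hit check is disconnected, so arrows draw even when traces miss.
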(event `self.ReceiveTick`
  (params (DeltaSeconds :type "Float (single-precision)"))
  (bind _sphere (`self.Sphere`))
  (bind _returnvalue (`SceneComponent.K2_GetComponentLocation` (`self.Sphere`)))
  (bind _sphereradius (`SphereComponent.SphereRadius` _sphere))
  (bind (_hit _hitresults) (`/Game/Blueprints/Global/CollisionHelpers.Overlap Sphere Helper` (`SceneComponent.K2_GetComponentLocation` _sphere) _sphereradius "ObjectTypeQuery1" "ForOneFrame"))
  (if _hit
    (for _array_element _hitresults
      (bind (_origin _translated_vector) (`/Game/Blueprints/Global/VectorHelpers.Translate Direction To World Location` _returnvalue (- (`.ImpactPoint` (`GameplayStatics.BreakHitResult` _array_element)) _returnvalue) _sphereradius true))
      (bind _outhit (`KismetSystemLibrary.LineTraceSingleForObjects` :`Start` _origin :`End` _translated_vector :`ObjectTypes` (`|MakeArray` "ObjectTypeQuery1" :!type "EObjectTypeQuery Enum") :`DrawDebugType` "ForOneFrame"))
      (bind (_origin_2 _translated_vector_2) (`/Game/Blueprints/Global/VectorHelpers.Translate Direction To World Location` _returnvalue (`.ImpactNormal` (`GameplayStatics.BreakHitResult` _outhit))))
      (`KismetSystemLibrary.DrawDebugArrow` _origin_2 _translated_vector_2 200.0 (struct :`G` 0.235459 :`B` 1.0 :`A` 1.0) 0.0 5.0))))

(fn `UserConstructionScript`)