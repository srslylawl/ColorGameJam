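; Enemy character with granny sounds that attacks and can bump through a child BumperComponent actor.
; The construction script passes force and held-item-removal settings to the bumper, whose collider starts disabled and toggles via EnableBump and DisableBump.
; Attack and AttackEnd swap looping-style AudioPlayer audio for an attack cue and, on authority only, mirror IsAttacking to the AI blackboard.
; OnStep plays footsteps at the mesh.
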(event `EnableBump`
  (bind _asbumper_component (cast `/Game/Blueprints/Environment/BumperComponent` (`ChildActorComponent.ChildActor` (`self.BumperComponent`))))
  (`PrimitiveComponent.SetCollisionEnabled` (`/Game/Blueprints/Environment/BumperComponent.Collider` _asbumper_component) "QueryAndPhysics"))

(event `DisableBump`
  (bind _asbumper_component (cast `/Game/Blueprints/Environment/BumperComponent` (`ChildActorComponent.ChildActor` (`self.BumperComponent`))))
  (`PrimitiveComponent.SetCollisionEnabled` (`/Game/Blueprints/Environment/BumperComponent.Collider` _asbumper_component) "NoCollision"))

(event `self.ReceiveBeginPlay`
  (`AudioComponent.Play` (`self.AudioPlayer`) 0.0)
  (`self.DisableBump`))

(event `OnStep`
  (`GameplayStatics.PlaySoundAtLocation` "/Game/SFX/Cues/Cue_GrannyStep.Cue_GrannyStep" (`SceneComponent.K2_GetComponentLocation` (`self.Mesh`)) (struct) 1.0 1.0 0.0 "/Game/SFX/GrannyAttenuation.GrannyAttenuation" null null))

(event `Attack`
  (if (not (`self.IsAttacking`))
    (`AudioComponent.Stop` (`self.AudioPlayer`))
    (set `self.IsAttacking` true)
    (`GameplayStatics.PlaySoundAtLocation` "/Game/SFX/Cues/Cue_GrannyAttack.Cue_GrannyAttack" (`SceneComponent.K2_GetComponentLocation` (`self.Mesh`)) (struct) 1.0 1.0 0.0 "/Game/SFX/EdibleAttenuation.EdibleAttenuation" null null)
    (`/Engine/EditorBlueprintResources/ActorMacros.Switch Has Authority`
      (:`Authority`
        (bind _asenemy_ai_controller (cast `/Game/Blueprints/AI/Enemy_AI_Controller` (`self.GetController`)))
        (`BlackboardComponent.SetValueAsBool` (`AIBlueprintHelperLibrary.GetBlackboard` _asenemy_ai_controller) "IsAttacking" true)))))

(event `AttackEnd`
  (set `self.IsAttacking` false)
  (`AudioComponent.Play` (`self.AudioPlayer`) 0.0)
  (`/Engine/EditorBlueprintResources/ActorMacros.Switch Has Authority`
    (:`Authority`
      (`BlackboardComponent.SetValueAsBool` (`AIBlueprintHelperLibrary.GetBlackboard` null) "IsAttacking" false))))

(fn `UserConstructionScript`
  (bind _asbumper_component (cast `/Game/Blueprints/Environment/BumperComponent` (`ChildActorComponent.ChildActor` (`self.BumperComponent`))))
  (set `/Game/Blueprints/Environment/BumperComponent.HorizontalForceOnly` (`self.HorizontalForceOnly`) _asbumper_component)
  (set `/Game/Blueprints/Environment/BumperComponent.ForceMultiplier` (`self.ForceMultiplier`) _asbumper_component)
  (set `/Game/Blueprints/Environment/BumperComponent.RemoveHeldItems` (`self.RemoveHeldItems`) _asbumper_component))