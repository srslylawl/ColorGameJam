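; Rat character that runs an endless patrol around a list of points while squeaking.
; On BeginPlay it registers itself as RatRef on the LevelGameMode, loops its run animation, applies its movement speed, and starts patrolling.
; PatrolToPoint uses AI MoveTo and calls itself on success, wrapping the index; a failed move is not handled.
; A looping timer plays the squeak at the mesh location with sound attenuation.
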(event `Squeak`
  (`GameplayStatics.PlaySoundAtLocation` "/Game/SFX/Cues/Cue_Rat.Cue_Rat" (`SceneComponent.K2_GetComponentLocation` (`self.Mesh`)) (struct) 1.0 1.0 0.0 "/Game/SFX/GrannyAttenuation.GrannyAttenuation" null null))

(event `self.ReceiveBeginPlay`
  (bind _aslevel_game_mode (cast `/Game/Blueprints/LevelGameMode` (`GameplayStatics.GetGameMode`)))
  (set `/Game/Blueprints/LevelGameMode.RatRef` self _aslevel_game_mode)
  (`SkeletalMeshComponent.PlayAnimation` (`self.Mesh`) "/Game/Characters/Heinrich/Heinrich_Run.Heinrich_Run" true)
  (set `CharacterMovementComponent.MaxWalkSpeed` (`self.MovementSpeed`) (`self.CharacterMovement`))
  (`self.PatrolToPoint`)
  (`KismetSystemLibrary.K2_SetTimerDelegate` (delegate `Squeak`) 0.5 true))

(event `PatrolToPoint`
  (`|AIMoveTo` self (0.0 0.0 0.0) (`|GetArrayItem` (`self.PatrolPoints`) (`self.PatrolPointIndex`))
    (:`OnSuccess`
      (if (>= (`self.PatrolPointIndex`) (- (`KismetArrayLibrary.Array_Length` (`self.PatrolPoints`)) 1))
        (set `self.PatrolPointIndex` 0)
        (else
          (`/Engine/EditorBlueprintResources/StandardMacros.IncrementInt` (`self.PatrolPointIndex`)
            (:`  `
              _))))
      (`self.PatrolToPoint`))))

(fn `UserConstructionScript`)