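; Bumper that knocks away overlapping actors implementing IBumpable, with a cooldown between bumps.
; On overlap it gets the object to bump from the interface, and BumpObject pushes it away from the Collider with a mass-independent impulse scaled by Force and ForceMultiplier, optionally horizontal only.
; BumpRelative, not called here, applies the same impulse and prints velocity-versus-direction debug data without using it.
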(event `self.ReceiveActorBeginOverlap`
  (params (OtherActor :type "Actor Object Reference"))
  (bind _asibumpable (cast `/Game/Blueprints/IBumpable` OtherActor))
  (if (`self.CanBump`)
    (bind _object (`/Game/Blueprints/IBumpable.GetObjectToBump` _asibumpable))
    (`self.BumpObject` _object)
    (set `self.CanBump` false)
    (`KismetSystemLibrary.Delay` (`self.Cooldown`))
    (set `self.CanBump` true)))

(fn `BumpObject`
  (params (BumpObject :type "PrimitiveComponent Object Reference"))
  (bind _returnvalue (- (`SceneComponent.K2_GetComponentLocation` BumpObject) (`SceneComponent.K2_GetComponentLocation` (`self.Collider`))))
  (if (`self.HorizontalForceOnly`)
    (set `self.ImpulseVector` (`KismetMathLibrary.Normal` (`KismetMathLibrary.MakeVector` (.x _returnvalue) (.y _returnvalue))))
    (else
      (set `self.ImpulseVector` (`KismetMathLibrary.Normal` _returnvalue))))
  (`PrimitiveComponent.AddImpulse` BumpObject (* (* (`self.ImpulseVector`) (`self.Force`)) (`self.ForceMultiplier`)) "None" true))

(fn `BumpRelative`
  (params (BumpObject :type "PrimitiveComponent Object Reference"))
  (bind _returnvalue (- (`SceneComponent.K2_GetComponentLocation` BumpObject) (`SceneComponent.K2_GetComponentLocation` (`self.Collider`))))
  (bind _returnvalue_2 (`PrimitiveComponent.GetPhysicsLinearVelocity` BumpObject "None"))
  (`KismetSystemLibrary.PrintString` (`KismetStringLibrary.Concat_StrStr` "Velocity: " (`KismetStringLibrary.Conv_VectorToString` _returnvalue_2) "Bump Dir: " (`KismetStringLibrary.Conv_VectorToString` _returnvalue) "Result: " (`KismetStringLibrary.Conv_DoubleToString` (`KismetMathLibrary.Dot_VectorVector` _returnvalue_2 _returnvalue))) true true (struct :`G` 0.66 :`B` 1.0 :`A` 1.0) 60.0)
  (if (`self.HorizontalForceOnly`)
    (set `self.ImpulseVector` (`KismetMathLibrary.Normal` (`KismetMathLibrary.MakeVector` (.x _returnvalue) (.y _returnvalue))))
    (else
      (set `self.ImpulseVector` (`KismetMathLibrary.Normal` _returnvalue))))
  (`PrimitiveComponent.AddImpulse` BumpObject (* (* (`self.ImpulseVector`) (`self.Force`)) (`self.ForceMultiplier`)) "None" true))

(fn `UserConstructionScript`)