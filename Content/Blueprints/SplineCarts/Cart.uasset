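; Cart actor that rides along the spline of a referenced spline tool actor, starting on BeginPlay when ActiveCart is set.
; The construction script applies the chosen mesh and, only if that mesh is valid, caches the tool's spline.
; MoveCart scales the CartMover timeline's play rate by Duration and starts it at CartStartOffset.
; Each update maps timeline alpha to distance along the spline, setting world location and rotation.
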(event `self.ReceiveBeginPlay`
  (if (`self.ActiveCart`)
    (`self.MoveCart`)))

(event `MoveCart`
  (bind _returnvalue (`KismetMathLibrary.Lerp` 0.0 (`SplineComponent.GetSplineLength` (`self.SplineRef`)) (`self.Alpha`)))
  (`/Engine/EditorBlueprintResources/StandardMacros.IsValid` (`self.SplineToolRef`)
    (:`Is Valid`
      (`TimelineComponent.SetPlayRate` (`self.CartMover`) (/ 1.0 (`self.Duration`)))
      (`TimelineComponent.SetNewTime` (`self.CartMover`) (`self.CartStartOffset`)) ; exactly the same thing as the "Set new time" pin in the timeline
      (bind (_direction _alpha) (`Timeline|CartMover`)
        (:`Update`
          (set `self.Alpha` _alpha)
          (`self.K2_SetActorLocationAndRotation` (`SplineComponent.GetLocationAtDistanceAlongSpline` (`self.SplineRef`) _returnvalue "World") (`SplineComponent.GetRotationAtDistanceAlongSpline` (`self.SplineRef`) _returnvalue "World")))))))

(fn `UserConstructionScript`
  (bind _mesh (`self.Mesh`))
  (bind _splinetoolref (`self.SplineToolRef`))
  (`/Engine/EditorBlueprintResources/StandardMacros.IsValid` _mesh
    (:`Is Valid`
      (`StaticMeshComponent.SetStaticMesh` (`self.CartMesh`) _mesh)
      (`/Engine/EditorBlueprintResources/StandardMacros.IsValid` _splinetoolref
        (:`Is Valid`
          (bind _spline (`/Game/Blueprints/SplineTool/SplineTool.GetSpline` _splinetoolref))
          (set `self.SplineRef` _spline))))))