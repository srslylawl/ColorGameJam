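; Multiplayer player character that moves a physics-driven Body with directional input and a Space-key jump impulse.
; On Tick, the locally controlled client sets horizontal velocity relative to Body facing, preserving vertical velocity, then sends velocity and transform through a C2S event.
; That event applies both directly to Body, trusting client state; jumps also go through C2S.
; An S2C velocity event exists but is not called here and ignores its transform.
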(event `C2S_UpdateVelocity`
  (params (Velocity :type "Vector Structure") (Transform :type "Transform Structure"))
  (bind _body (`self.Body`))
  (`PrimitiveComponent.SetPhysicsLinearVelocity` _body Velocity false "None")
  (`SceneComponent.K2_SetWorldTransform` _body Transform true true))

(event `self.ReceiveTick`
  (params (DeltaSeconds :type "Float (single-precision)"))
  (bind _body (`self.Body`))
  (if (`self.IsLocallyControlled`)
    (`self.HandleDirectionalInput`)
    (`self.SetVelocity` (`self.MovementInput`))
    (bind _returnvalue (`PrimitiveComponent.GetPhysicsLinearVelocity` _body "None"))
    (`self.C2S_UpdateVelocity` _returnvalue (`SceneComponent.K2_GetComponentToWorld` _body))))

(event `S2C_UpdateVelocity`
  (params (MovementInput :type "Vector Structure") (Transform :type "Transform Structure"))
  (`self.SetVelocity` MovementInput))

(event `C2S_Jump`
  (`self.Jump`))

(event `Key|SpaceBar`
  (params (Key :type "Key Structure"))
  (:`Pressed`
    (`self.Jump`)
    (`self.C2S_Jump`)
    (`self.DebugString` "pressed Space")))

(event `DebugString`
  (params (string :type String))
  (`KismetSystemLibrary.PrintString` (`KismetStringLibrary.Concat_StrStr` "Player " (`KismetStringLibrary.Conv_IntToString` (`self.PlayerNumber`)) " " string)))

(fn `HandleDirectionalInput`
  (set `self.MovementInput` (`KismetMathLibrary.Normal` (`KismetMathLibrary.MakeVector` (`self.GetInputAxisValue`) (`self.GetInputAxisValue`))))
  (return))

(fn `Jump`
  (`PrimitiveComponent.AddImpulse` (`self.Body`) (* (0.0 0.0 1.0) 500.0) "None" true))

(fn `SetVelocity`
  (params (MovementInput :type "Vector Structure"))
  (locals (MoveSpeed :type "Float (double-precision)"))
  (bind _body (`self.Body`))
  (bind _output_get (set `local.MoveSpeed` 500.0))
  (bind _returnvalue (`PrimitiveComponent.GetPhysicsLinearVelocity` _body "None"))
  (bind (_returnvalue_x _returnvalue_y) (`KismetMathLibrary.BreakVector` (* (+ (* (`SceneComponent.GetForwardVector` _body) MovementInput_X) (* (`SceneComponent.GetRightVector` _body) MovementInput_Y)) _output_get)))
  (`PrimitiveComponent.SetPhysicsLinearVelocity` _body (`KismetMathLibrary.MakeVector` _returnvalue_x _returnvalue_y (.z _returnvalue)) false "None"))

(fn `UserConstructionScript`)