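; Multiplayer game mode that tracks edible collection as level progress and handles the win.
; Spawn and collect handlers update running totals and broadcast progress, measured as collected over EdiblesNeeded and capped at 1.
; Full progress triggers a one-time win: winning screen, sound and mouse cursor, for player controller 0.
; Player start selection uses each MP_PlayerController's PlayerNumber as an index into all PlayerStart actors.
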(fn `ChoosePlayerStartOverride`
  (params (Object :type "PlayerController Object Reference"))
  (returns (ReturnValue :type "Actor Object Reference"))
  (bind _asmp_player_controller (cast `/Game/Blueprints/MP/MP_PlayerController` Object))
  (bind _outactors (`GameplayStatics.GetAllActorsOfClass` "/Script/Engine.PlayerStart"))
  (return (`|GetArrayItem` _outactors (`/Game/Blueprints/MP/MP_PlayerController.PlayerNumber` _asmp_player_controller))))

(fn `GetProgress`
  (returns (ProgressPercent :type "Float (double-precision)"))
  (locals (LevelProgress :type "Float (double-precision)") (RequiredPercent :type "Float (double-precision)" :default 0.1))
  (if (> (`self.TotalEdiblesSpawned`) 0)
    (set `local.LevelProgress` (`KismetMathLibrary.FMin` (/ (`KismetMathLibrary.Conv_IntToDouble` (`self.TotalEdiblesCollected`)) (`KismetMathLibrary.Conv_IntToDouble` (`self.EdiblesNeeded`))) 1.0))
    (else
      (set `local.LevelProgress` 0.0)))
  (return (`local.LevelProgress`)))

(fn `OnEdibleCollected`
  (params (Amount :type Integer))
  (bind _progresspercent (`self.GetProgress`))
  (set `self.TotalEdiblesCollected` (+ Amount (`self.TotalEdiblesCollected`)))
  (`self.ProgressUpdate` _progresspercent)
  (if (and (not (`self.GameWon`)) (>= _progresspercent 1.0))
    (set `self.GameWon` true)
    (bind _returnvalue (`|CreateWidget` "/Game/Blueprints/HUD/WinningScreen.WinningScreen_C" (`GameplayStatics.GetPlayerController` 0)))
    (`UserWidget.AddToViewport` _returnvalue 0)
    (`GameplayStatics.PlaySound2D` "/Game/SFX/Cues/Cue_Win.Cue_Win" 1.0 1.0 0.0 null null)
    (set `PlayerController.bShowMouseCursor` true (`GameplayStatics.GetPlayerController` 0))))

(fn `OnEdibleSpawned`
  (params (Amount :type Integer))
  (set `self.TotalEdiblesSpawned` (+ Amount (`self.TotalEdiblesSpawned`)))
  (`self.ProgressUpdate` (`self.GetProgress`)))

(fn `UserConstructionScript`)