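; Multiplayer player controller that spawns each player's Slimey pawn and keeps lobby player info updated.
; On BeginPlay under MultiplayerGameMode, it increments the player count, spawns Slimey at the player start named by that number, and possesses it.
; Under LobbyGameMode, BeginPlay and EndPlay both copy the SaveOptions player name into MP_PlayerState, then trigger the lobby's player update.
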(event `ServerNameChange`
  (bind _returnvalue (`GameplayStatics.LoadGameFromSlot` "SaveOptions"))
  (bind _assave_options (cast `/Game/Blueprints/Menu/SaveOptions` _returnvalue))
  (bind _asmp_player_state (cast `/Game/Blueprints/MP/MP_PlayerState` (`self.PlayerState`)))
  (set `/Game/Blueprints/MP/MP_PlayerState.PlayerName` (`/Game/Blueprints/Menu/SaveOptions.PlayerName` _assave_options) _asmp_player_state))

(event `self.ReceiveBeginPlay`
  (bind _returnvalue (`GameplayStatics.GetGameMode`))
  (`|ExecutionSequence`
    (:`then_0`
      (bind _asmultiplayer_game_mode (cast `/Game/Blueprints/MP/MultiplayerGameMode` _returnvalue))
      (bind _output_get (set `/Game/Blueprints/MP/MultiplayerGameMode.PlayerCount` (+ (stale _output_get) 1) _asmultiplayer_game_mode))
      (bind _output_get_2 (set `self.PlayerNumber` _output_get))
      (bind _returnvalue_2 (`|SpawnActorFromClass` "/Game/Blueprints/Character/Slimey.Slimey_C" (`self.GetTransform` (`GameModeBase.K2_FindPlayerStart` _asmultiplayer_game_mode self (`KismetStringLibrary.Conv_IntToString` _output_get_2))) "AdjustIfPossibleButAlwaysSpawn" "OverrideRootScale" null null))
      (`self.Possess` _returnvalue_2)
      (set `/Game/Blueprints/Character/Slimey.Possessed` true _returnvalue_2))
    (:`then_1`
      (bind _aslobby_game_mode (cast `/Game/Blueprints/MP/LobbyGameMode` _returnvalue :!label _label))
      (`self.ServerNameChange`)
      (`/Game/Blueprints/MP/LobbyGameMode.OnPlayerUpdate` _aslobby_game_mode))))

(event `self.ReceiveEndPlay`
  (params (EndPlayReason :type "EEndPlayReason Enum" :default "Destroyed"))
  (goto _label))

(fn `UserConstructionScript`)