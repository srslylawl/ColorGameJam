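; Game state for the Slimey game that tracks collected edibles and triggers victory when the goal is reached.
; OnEdibleCollected adds to the count, reports progress as collected over needed via CallProgressUpdate, and fires victory once, guarded by GameWon.
; Victory adds the winning screen widget to the viewport, plays a win sound and shows the mouse cursor.
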(fn `GetProgress`
  (returns (progressPercent :type "Float (double-precision)"))
  (return (`KismetMathLibrary.SafeDivide` (`KismetMathLibrary.Conv_IntToDouble` (`self.EdiblesCollected`)) (`KismetMathLibrary.Conv_IntToDouble` (`self.EdiblesNeeded`)))))

(fn `OnEdibleCollected`
  (params (Amount :type Integer))
  (bind _progresspercent (`self.GetProgress`))
  (bind _output_get (set `self.EdiblesCollected` (+ (stale _output_get) Amount)))
  (`self.ProgressUpdate` _progresspercent)
  (if (and (>= _progresspercent 1.0) (not (`self.GameWon`)))
    (set `self.GameWon` true)
    (`self.TriggerVictory`)))

(fn `TriggerVictory`
  (bind _returnvalue (`|CreateWidget` "/Game/Blueprints/HUD/Game_WinningScreen.Game_WinningScreen_C" (`GameplayStatics.GetPlayerController` 0)))
  (`UserWidget.AddToViewport` _returnvalue 0)
  (`GameplayStatics.PlaySound2D` "/Game/SFX/Cues/Cue_Win.Cue_Win" 1.0 1.0 0.0 null null)
  (set `PlayerController.bShowMouseCursor` true (`GameplayStatics.GetPlayerController` 0)))

(fn `UserConstructionScript`)