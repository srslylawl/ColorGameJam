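; Spline tool actor that lays a chosen static mesh along an editable spline, open or closed, as a chain of colliding spline mesh components.
; The construction script calls Update, which divides the spline into sections of SectionLength multiplied by the actor's scale on the chosen forward axis.
; Each section takes position, scale and roll from the spline, with tangents clamped to section length.
; Closed loops add a segment back to the start.
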(event `self.ReceiveBeginPlay`)

(fn `AssignMeshValues`
  (params (StartPos :type "Float (double-precision)") (EndPos :type "Float (double-precision)") (Length :type "Float (double-precision)") (UpdateMesh :type Boolean) (SetTransform :type Boolean) (Transform :type "Transform Structure"))
  (bind _spline (`self.Spline`))
  (bind _length (`local.Length`))
  (bind _returnvalue (`AddComponent|NODE_AddSplineMeshComponent-2` :`bManualAttachment` SetTransform :`RelativeTransform` Transform))
  (bind _output_get (set `self.SplineMeshComponent` _returnvalue))
  (`StaticMeshComponent.SetStaticMesh` _output_get (`self.MeshToSpline`))
  (`PrimitiveComponent.SetCollisionResponseToAllChannels` _output_get "ECR_Block")
  (`PrimitiveComponent.SetCollisionEnabled` _output_get "QueryAndPhysics")
  (`SplineMeshComponent.SetForwardAxis` _output_get (`self.ForwardAxis`) false)
  (`SplineMeshComponent.SetStartScale` _output_get (`KismetMathLibrary.Conv_VectorToVector2D` (`SplineComponent.GetScaleAtDistanceAlongSpline` _spline StartPos)) false)
  (`SplineMeshComponent.SetEndScale` _output_get (`KismetMathLibrary.Conv_VectorToVector2D` (`SplineComponent.GetScaleAtDistanceAlongSpline` _spline EndPos)) false)
  (`SplineMeshComponent.SetStartRoll` _output_get (`KismetMathLibrary.DegreesToRadians` (`SplineComponent.GetRollAtDistanceAlongSpline` _spline StartPos "Local")) false)
  (`SplineMeshComponent.SetEndRoll` _output_get (`KismetMathLibrary.DegreesToRadians` (`SplineComponent.GetRollAtDistanceAlongSpline` _spline EndPos "Local")) false)
  (`SplineMeshComponent.SetStartAndEnd` _output_get (`SplineComponent.GetLocationAtDistanceAlongSpline` _spline StartPos "Local") (`KismetMathLibrary.ClampVectorSize` (`SplineComponent.GetTangentAtDistanceAlongSpline` _spline StartPos "Local") 0.0 _length) (`SplineComponent.GetLocationAtDistanceAlongSpline` _spline EndPos "Local") (`KismetMathLibrary.ClampVectorSize` (`SplineComponent.GetTangentAtDistanceAlongSpline` _spline EndPos "Local") 0.0 _length) (`local.UpdateMesh`)))

(fn `GetSpline`
  (returns (Spline :type "SplineComponent Object Reference"))
  (return (`self.Spline`)))

(fn `SetupMeshPart`
  (params (index :type Integer) (length :type "Float (double-precision)") (isLast :type Boolean))
  (`self.AssignMeshValues` (* index length) (* (+ index 1) length) length isLast))

(fn `Update`
  (locals (LocalLength :type "Float (double-precision)"))
  (bind (_returnvalue_x _returnvalue_y _returnvalue_z) (`KismetMathLibrary.BreakVector` (`self.GetActorScale3D`)))
  (bind _closedloop (`self.ClosedLoop`))
  (bind _output_get (set `local.LocalLength` (* (select `ESplineMeshAxis` (`self.ForwardAxis`) :`X` _returnvalue_x :`Y` _returnvalue_y :`Z` _returnvalue_z) (`self.SectionLength`))))
  (`SplineComponent.SetClosedLoop` (`self.Spline`) (`self.ClosedLoop`) true)
  (bind _returnvalue (`KismetMathLibrary.FTrunc` (/ (`SplineComponent.GetSplineLength` (`self.Spline`)) _output_get)))
  (for _index (range (+ _returnvalue 1))
    (`self.SetupMeshPart` _index _output_get (`KismetMathLibrary.BooleanNAND` (== _returnvalue _index) _closedloop)))
  (if _closedloop
    (`self.AssignMeshValues` (* _index _output_get) 0.0 _output_get true)))

(fn `UserConstructionScript`
  (locals (LocalLength :type "Float (double-precision)"))
  (`self.Update`))