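; BPF_PID is a Blueprint function that computes a PID controller output from a current and desired value.
; It sums the gain-weighted proportional, integral and derivative terms plus a bias, scaled to frame time through DeltaTime.
; The caller holds the state: Integral and ErrorPrior are updated by reference on each call.
; Error is current minus desired, with no integral clamp or zero-DeltaTime guard.
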(fn `PIDCalculation`
  (params (CurrentValue :type "Float (double-precision)") (DesiredValue :type "Float (double-precision)") (P :type "Float (double-precision)") (I :type "Float (double-precision)") (D :type "Float (double-precision)") (Bias :type "Float (double-precision)") (DeltaTime :type "Float (double-precision)") (Integral :type "Float (double-precision) (by ref)") (ErrorPrior :type "Float (double-precision) (by ref)"))
  (returns (OutForce :type "Float (double-precision)"))
  (locals (pIntegral :type "Float (double-precision)") (pErrorPrior :type "Float (double-precision)") (pError :type "Float (double-precision)") (pDerivative :type "Float (double-precision)"))
  (set `local.pErrorPrior` ErrorPrior)
  (set `local.pIntegral` Integral)
  (bind _output_get (set `local.pError` (- CurrentValue DesiredValue)))
  (set `local.pIntegral` (+ (`local.pIntegral`) (* _output_get DeltaTime)))
  (set `local.pDerivative` (/ (- _output_get (`local.pErrorPrior`)) DeltaTime))
  (`|VariableSetRef` Integral (`local.pIntegral`))
  (`|VariableSetRef` ErrorPrior (`local.pError`))
  (return (+ (* P (`local.pError`)) (* (`local.pIntegral`) I) (* (`local.pDerivative`) D) Bias)))