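; CollisionHelpers is a Blueprint helper whose OverlapSphereHelper function tests for objects of a given type around a location.
; It emulates a sphere overlap by running a complex multi sphere trace from that location along each offset in a Directions array, with optional debug drawing.
; It ORs the trace results into one hit flag and merges the hit results into an array with AddUnique, returning both.
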(fn `Overlap Sphere Helper`
  (params (Location :type "Vector Structure") (Radius :type "Float (double-precision)") (ObjectType :type "EObjectTypeQuery Enum" :default "ObjectTypeQuery1") (DrawDebug :type "EDrawDebugTrace Enum" :default "None"))
  (returns (Hit :type Boolean) (HitResults :type "Array of HitResult Structure"))
  (locals (Directions :type "Array of Vector Structure") (Result :type Boolean) (Endresult :type "Array of HitResult Structure"))
  (for _array_element (`local.Directions`)
    (bind (_outhits _returnvalue) (`KismetSystemLibrary.SphereTraceMultiForObjects` :`Start` Location :`End` (+ _array_element Location) :`Radius` Radius :`ObjectTypes` (`|MakeArray` ObjectType) :`bTraceComplex` true :`DrawDebugType` DrawDebug))
    (bind _output_get (set `local.Result` (or (stale _output_get) _returnvalue)))
    (for _array_element_2 _outhits
      (`KismetArrayLibrary.Array_AddUnique` (`local.Endresult`) _array_element_2)))
  (return _output_get (`local.Endresult`)))