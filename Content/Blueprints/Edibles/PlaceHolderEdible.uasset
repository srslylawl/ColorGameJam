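; Level placeholder for edibles that swaps itself for an EdibleObject on BeginPlay and then destroys itself once a data table row is found.
; The construction script previews either the chosen row's mesh and size or a Small, Medium or Large bounds mesh.
; At runtime it passes the spawned object either that specific row or a random size-matched one, picking names from SpecificObject's table but reading the row from EdibleAssetList.
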(event `self.ReceiveBeginPlay`
  (bind (_specificobject_datatable _specificobject_rowname) (break `DataTableRowHandle` (`self.SpecificObject`)))
  (if (`self.UseSpecificObject`)
    (bind _returnvalue (`|GetDataTableRow` _specificobject_datatable _specificobject_rowname)
      (:`then`
        (bind _returnvalue_2 (`|SpawnActorFromClass` "/Game/Blueprints/Edibles/EdibleObject.EdibleObject_C" (`self.GetTransform`) "Undefined" "OverrideRootScale" null (struct) null))
        (`/Game/Blueprints/Edibles/EdibleObject.InitiateFromPlaceholder` _returnvalue_2 _returnvalue)
        (`self.K2_DestroyActor`)))
    (else
      (bind _ediblerowname (`self.GetRandomAssetDataFromSize` (`self.Size`)))
      (bind _returnvalue_3 (`|SpawnActorFromClass` "/Game/Blueprints/Edibles/EdibleObject.EdibleObject_C" (`self.GetTransform`) "Undefined" "OverrideRootScale" null (struct) null))
      (bind _returnvalue_4 (`|GetDataTableRow` "/Game/Blueprints/Edibles/EdibleAssetList.EdibleAssetList" _ediblerowname)
        (:`then`
          (`/Game/Blueprints/Edibles/EdibleObject.InitiateFromPlaceholder` _returnvalue_3 _returnvalue_4)
          (`self.K2_DestroyActor`))))))

(fn `GetRandomAssetDataFromSize`
  (params (Size :type "/Game/Blueprints/Edibles/EdibleSize Enum" :default "NewEnumerator0"))
  (returns (EdibleRowName :type Name))
  (locals (EdibleDataTemp :type "Array of Name"))
  (bind _specificobject_datatable (break `DataTableRowHandle` (`self.SpecificObject`)))
  (bind _outrownames (`DataTableFunctionLibrary.GetDataTableRowNames` _specificobject_datatable))
  ;[1 1 1] ForeachLoop
  (for _array_element _outrownames
    (bind _returnvalue (`|GetDataTableRow` _specificobject_datatable _array_element)
      (:`then`
        (if (`|EnumEquality` (`.EdibleSize_11_1B9E9E6E4B5C05300078098D0B0A1A8C` (break `/Game/Blueprints/Structs/EdibleAssetData` _returnvalue)) Size)
          (`KismetArrayLibrary.Array_Add` (`local.EdibleDataTemp`) _array_element)))))
  ;[1 1 1] return random mesh by size
  (return (`KismetArrayLibrary.Array_Random` (`local.EdibleDataTemp`))))

(fn `UserConstructionScript`
  (bind (_specificobject_datatable _specificobject_rowname) (break `DataTableRowHandle` (`self.SpecificObject`)))
  (bind _staticmesh (`self.StaticMesh`))
  (if (`self.UseSpecificObject`)
    ;[1 1 1] Use specific object, selected by row
    (bind _returnvalue (`|GetDataTableRow` _specificobject_datatable _specificobject_rowname)
      (:`then`
        (bind (_ediblesize _mesh) (break `/Game/Blueprints/Structs/EdibleAssetData` _returnvalue))
        (set `self.Size` _ediblesize)
        (`StaticMeshComponent.SetStaticMesh` _staticmesh _mesh)))
    (else
      ;[1 1 1] Get Placeholder object by given size
      (switch `/Game/Blueprints/Edibles/EdibleSize` (`self.Size`)
        (:`NewEnumerator0`
          (`StaticMeshComponent.SetStaticMesh` _staticmesh "/Game/Meshes/EdibleBounds_SMALL.EdibleBounds_SMALL"))
        (:`NewEnumerator1`
          (`StaticMeshComponent.SetStaticMesh` _staticmesh "/Game/Meshes/EdibleBounds_MEDIUM.EdibleBounds_MEDIUM"))
        (:`NewEnumerator2`
          (`StaticMeshComponent.SetStaticMesh` _staticmesh "/Game/Meshes/EdibleBounds_LARGE.EdibleBounds_LARGE"))))))