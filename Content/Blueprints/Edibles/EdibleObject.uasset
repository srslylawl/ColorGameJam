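; EdibleObject is a colored edible pickup that hands itself to the MainCharacter on overlap while pickup is allowed, re-enabling pickup when that overlap ends.
; It spawns from a placeholder's asset data with a random color or from vomit with its existing reference.
; Color selects both material and collision object channel.
; Placeholder spawns and collection report size-based amounts to LevelGameMode, and collection destroys the actor.
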(event `self.StaticMeshComponent.OnComponentBeginOverlap`
  (params (OverlappedComponent :type "PrimitiveComponent Object Reference") (OtherActor :type "Actor Object Reference") (OtherComp :type "PrimitiveComponent Object Reference") (OtherBodyIndex :type Integer) (bFromSweep :type Boolean) (SweepResult :type "HitResult Structure (by ref)"))
  (bind _asmain_character (cast `/Game/Blueprints/Character/MainCharacter` OtherActor))
  (if (`self.CanBePickedUp`)
    (`/Game/Blueprints/Character/MainCharacter.PickupObject` _asmain_character self)))

(event `self.StaticMeshComponent.OnComponentEndOverlap`
  (params (OverlappedComponent :type "PrimitiveComponent Object Reference") (OtherActor :type "Actor Object Reference") (OtherComp :type "PrimitiveComponent Object Reference") (OtherBodyIndex :type Integer))
  (cast `/Game/Blueprints/Character/MainCharacter` OtherActor)
  (set `self.CanBePickedUp` true))

(fn `Create`
  (params (EdibleIngameReference :type "/Game/Blueprints/Edibles/EdibleIngameReference Structure"))
  (bind (_edibleassetdata _color) (break `/Game/Blueprints/Edibles/EdibleIngameReference` EdibleIngameReference))
  (bind _staticmeshcomponent (`self.StaticMeshComponent`))
  (`StaticMeshComponent.SetStaticMesh` _staticmeshcomponent (`.Mesh_10_671EBB36453F2E86F5461EB0A55AE109` (break `/Game/Blueprints/Edibles/EdibleAssetData` _edibleassetdata)))
  (`self.SetMaterialByColor` _color _edibleassetdata)
  (`PrimitiveComponent.SetCollisionObjectType` _staticmeshcomponent (select `/Game/Blueprints/Edibles/EdibleColor` _color :`NewEnumerator0` "ECC_GameTraceChannel1" :`NewEnumerator1` "ECC_GameTraceChannel2" :`NewEnumerator2` "ECC_GameTraceChannel3" :!type "ECollisionChannel Enum")))

(fn `GetRandomColor`
  (returns (Color :type "/Game/Blueprints/Edibles/EdibleColor Enum"))
  (return (cast `/Game/Blueprints/Edibles/EdibleColor` (`KismetMathLibrary.Conv_IntToByte` (`KismetMathLibrary.RandomInteger` 3)))))

(fn `IncrementLevelAmount`
  (params (Amount :type Integer))
  (bind _aslevel_game_mode (cast `/Game/Blueprints/LevelGameMode` (`GameplayStatics.GetGameMode`)))
  (`/Game/Blueprints/LevelGameMode.OnEdibleSpawned` _aslevel_game_mode Amount))

(fn `Initiate From Vomit`
  (`self.Create` (`self.EdibleIngameRef`)))

(fn `InitiateFromPlaceholder`
  (params (EdibleAssetData :type "/Game/Blueprints/Edibles/EdibleAssetData Structure"))
  (bind _color (`self.GetRandomColor`))
  (bind _output_get (set `self.EdibleIngameRef` (make `/Game/Blueprints/Edibles/EdibleIngameReference` EdibleAssetData _color)))
  (`self.Create` _output_get)
  (`self.IncrementLevelAmount` (+ (`KismetMathLibrary.Conv_ByteToInt` (`.EdibleSize_11_1B9E9E6E4B5C05300078098D0B0A1A8C` (break `/Game/Blueprints/Edibles/EdibleAssetData` EdibleAssetData))) 1))
  (set `self.CanBePickedUp` true))

(fn `SetMaterialByColor`
  (params (Color :type "/Game/Blueprints/Edibles/EdibleColor Enum" :default "NewEnumerator0") (EdibleAssetData :type "/Game/Blueprints/Edibles/EdibleAssetData Structure"))
  (bind (_ediblesize _mesh _redcolorinstance _bluecolorinstance _greencolorinstance) (break `/Game/Blueprints/Edibles/EdibleAssetData` EdibleAssetData))
  (bind _staticmeshcomponent (`self.StaticMeshComponent`))
  (switch `/Game/Blueprints/Edibles/EdibleColor` Color
    (:`NewEnumerator0`
      (`PrimitiveComponent.SetMaterial` _staticmeshcomponent 0 _redcolorinstance))
    (:`NewEnumerator1`
      (`PrimitiveComponent.SetMaterial` _staticmeshcomponent 0 _bluecolorinstance))
    (:`NewEnumerator2`
      (`PrimitiveComponent.SetMaterial` _staticmeshcomponent 0 _greencolorinstance))))

(fn `TriggerCollected`
  (bind _aslevel_game_mode (cast `/Game/Blueprints/LevelGameMode` (`GameplayStatics.GetGameMode`)))
  (`/Game/Blueprints/LevelGameMode.OnEdibleCollected` _aslevel_game_mode (+ (`KismetMathLibrary.Conv_ByteToInt` (`.EdibleSize_11_1B9E9E6E4B5C05300078098D0B0A1A8C` (break `/Game/Blueprints/Edibles/EdibleAssetData` (`.EdibleAssetData_21_FE1CFB6645C15924EF370CAF3CAE3B33` (break `/Game/Blueprints/Edibles/EdibleIngameReference` (`self.EdibleIngameRef`)))))) 1))
  (`self.K2_DestroyActor`))

(fn `UserConstructionScript`)