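; EdibleObject is a collectible actor that adds to a per-color count on the MainCharacter when the character overlaps its static mesh.
; On overlap it switches on its color enum and increments the Red, Blue or Green counter.
; Blue and Green then destroy the actor, while Red does not.
; BeginPlay caches the player character, used only by unconnected ObjectsEaten logging code; an EdibleData assignment also never runs.
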(event `self.ReceiveBeginPlay`
  (bind _asmain_character (cast `/Game/Blueprints/MainCharacter` (`GameplayStatics.GetPlayerPawn` 0)))
  (set `self.CharacterReference` _asmain_character))

(event `self.StaticMeshComponent.OnComponentBeginOverlap`
  (params (OverlappedComponent :type "PrimitiveComponent Object Reference") (OtherActor :type "Actor Object Reference") (OtherComp :type "PrimitiveComponent Object Reference") (OtherBodyIndex :type Integer) (bFromSweep :type Boolean) (SweepResult :type "HitResult Structure (by ref)"))
  (switch `/Game/Blueprints/ColorEnums` (`self.ObjectColorEnum`)
    (:`NewEnumerator0`
      (bind _asmain_character (cast `/Game/Blueprints/MainCharacter` OtherActor))
      (`/Engine/EditorBlueprintResources/StandardMacros.IncrementInt` (`/Game/Blueprints/MainCharacter.RedObjectsCollected` _asmain_character)))
    (:`NewEnumerator1`
      (bind _asmain_character_2 (cast `/Game/Blueprints/MainCharacter` OtherActor))
      (`/Engine/EditorBlueprintResources/StandardMacros.IncrementInt` (`/Game/Blueprints/MainCharacter.BlueObjectsCollected` _asmain_character_2)
        (:`  `
          (`self.K2_DestroyActor`))))
    (:`NewEnumerator2`
      (bind _asmain_character_3 (cast `/Game/Blueprints/MainCharacter` OtherActor))
      (`/Engine/EditorBlueprintResources/StandardMacros.IncrementInt` (`/Game/Blueprints/MainCharacter.GreenObjectsCollected` _asmain_character_3)
        (:`  `
          (`self.K2_DestroyActor`))))))

(fn `UserConstructionScript`)